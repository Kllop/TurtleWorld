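; TurtleOne is a pawn that walks to a target actor on request, then explodes and destroys itself on arrival.
; GotoLocation stores the target and start location, then MoveToLocation drives the pawn with AI Move To.
; While moving, it attaches a smoke emitter to its capsule, plays a walk sound and sets a one-second timer.
; On success, it spawns an explosion effect and sound before removing itself.
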(event `self.ReceiveBeginPlay`)

(event `/Game/Blueprints/Interface/InterectableSpawnObject.GoToLocation`
  (params (TargetActor :type "Actor Object Reference"))
  (set `self.TargetActor` TargetActor)
  (set `self.StartLocation` (`self.K2_GetActorLocation`))
  (`self.MoveToLocation`))

(event `MoveToLocation`
  (`self.BeginMovment`)
  (`|AIMoveTo` self (0.0 0.0 0.0) (`self.TargetActor`)
    (:`then`
      (`self.Moving`))
    (:`OnSuccess`
      (`self.FinishMovment`))))

(fn `BeginMovment`)

(fn `FinishMovment`
  (`GameplayStatics.SpawnSoundAtLocation` "/Game/Sounds/djoker-fokus-s-karandasom-temniy-ricar-dark-knight__videomega__mp3cut_net__Cue.djoker-fokus-s-karandasom-temniy-ricar-dark-knight__videomega__mp3cut_net__Cue" (`self.K2_GetActorLocation`) (struct) 1.0 1.0 0.0 null null)
  (`GameplayStatics.SpawnEmitterAtLocation` "/Game/VFX/Particles/P_Explosion.P_Explosion" (`self.K2_GetActorLocation`))
  (`self.K2_DestroyActor`))

(fn `Moving`
  (`self.SpawnWalkEffect`)
  (`self.SpawnWalkSound`))

(fn `SpawnWalkEffect`
  (`/Engine/EditorBlueprintResources/StandardMacros.IsValid` (`self.WalkEffect`)
    (:`Is Valid`
      _)
    (:`Is Not Valid`
      (bind _returnvalue (`GameplayStatics.SpawnEmitterAttached` "/Game/VFX/Particles/P_Smoke.P_Smoke" (`self.CapsuleComponent`) "None" (-50.0 0.0 -50.0) (struct :`Pitch` -50.0 :`Yaw` -180.0)))
      (set `self.WalkEffect` _returnvalue)))
  (return))

(fn `SpawnWalkSound`
  (`GameplayStatics.SpawnSoundAtLocation` "/Game/Sounds/Walk.Walk" (`self.K2_GetActorLocation`) (struct) 1.0 1.0 0.0 null null)
  (bind _returnvalue (`KismetSystemLibrary.K2_SetTimerDelegate` (`|CreateDelegate` :!event `SpawnWalkSound`) 1.0))
  (set `self.SpawmWalkSoundHandle` _returnvalue))

(fn `UserConstructionScript`)