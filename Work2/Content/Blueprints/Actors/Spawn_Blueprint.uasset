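; Spawn point actor that creates a Turtle through its SpawnTurtle function, which runs only when the Turtle class is valid.
; It spawns the turtle at its own location, ignoring collisions, and sends it a GoToLocation message with the Spawn value.
; Each spawn plays a sound cue and attaches a steam particle effect to the actor's root.
; The event graph and construction script hold no logic.
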(fn `SpawnTurtle`
  (if (`KismetSystemLibrary.IsValidClass` (`self.Turtle`))
    (bind _returnvalue (`|SpawnActorFromClass` (`self.Turtle`) (`KismetMathLibrary.Conv_VectorToTransform` (`self.K2_GetActorLocation`)) "AlwaysSpawn" "OverrideRootScale" null null))
    (message `/Game/Blueprints/Interface/InterectableSpawnObject.GoToLocation` _returnvalue (`self.Spawn`))
    (`GameplayStatics.SpawnSoundAtLocation` "/Game/Sounds/oan1_Cue.oan1_Cue" (`self.K2_GetActorLocation`) (struct) 1.0 1.0 0.0 null null)
    (`GameplayStatics.SpawnEmitterAttached` "/Game/VFX/Particles/P_Steam_Lit.P_Steam_Lit" (`self.DefaultSceneRoot`) "None" (0.0 0.0 0.0) (struct :`Pitch` 90.0))
    (return)))

(fn `UserConstructionScript`)