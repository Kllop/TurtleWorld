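; TurtleTwo is a child turtle actor that customizes the inherited begin, stop and finish movement functions.
; BeginMovment calls the parent and starts a one-shot delay timer, which FinishMovment clears before calling the parent.
; StopMovment halts the controller without calling the parent, clears the walk sound timer, destroys the walk effect and starts a short timer.
; Both timers' callback targets are unspecified, and the event graph is unused.
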(fn `BeginMovment`
  (`parent.BeginMovment`)
  (bind _returnvalue (`KismetSystemLibrary.K2_SetTimerDelegate` (`|CreateDelegate` :!event `StopMovment`) 1.0))
  (set `self.DelayMovmentHandler` _returnvalue))

(fn `FinishMovment`
  (`KismetSystemLibrary.K2_ClearAndInvalidateTimerHandle` (`self.DelayMovmentHandler`))
  (`parent.FinishMovment`))

(fn `StopMovment`
  (`Controller.StopMovement` (`self.GetController`))
  (`KismetSystemLibrary.K2_SetTimerDelegate` (`|CreateDelegate` :!event `MoveToLocation`) 0.5)
  (`KismetSystemLibrary.K2_ClearAndInvalidateTimerHandle` (`self.SpawmWalkSoundHandle`))
  (`ActorComponent.K2_DestroyComponent` (`self.WalkEffect`)))

(fn `UserConstructionScript`
  (`parent.UserConstructionScript`))